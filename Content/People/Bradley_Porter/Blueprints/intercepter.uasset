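; Interceptor pawn that wanders at random and is wired to pursue a mover actor.
; BeginPlay checks the target once, then repeats simple move orders at random delays, either toward a mover or to random reachable points nearby.
; A SightSphere overlap stores the mover as target but never switches loops.
; The chase reads a separate cast result that never executes, not the stored target.
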(event OnComponentBeginOverlap(sightsphere)
  (params (OtherActor :type Actor%20Object%20Reference) (OtherComp :type Primitive%20Component%20Object%20Reference) (OtherBodyIndex :type Integer) (bFromSweep :type Boolean) (SweepResult :type Hit%20Result%20Structure%20%28by%20ref%29))
  (bind _asmover (Utilities|Casting|CastTomover OtherActor))
  (Variables|Default|Setmoverletarget _asmover))

(event EventBeginPlay
  (if (Utilities|IsValid (Variables|Default|Getmoverletarget))
    (AI|Navigation|SimpleMovetoLocation (Pawn|GetController) (Transformation|GetActorLocation (stale _asmover)) :!label _label)
    (Utilities|FlowControl|Delay (Math|Random|RandomFloatinRange 1.0 15.0))
    (goto _label)
    (else
      (AI|Navigation|SimpleMovetoLocation (Pawn|GetController) (AI|Navigation|GetRandomReachablePointinRadius (Transformation|GetActorLocation) (Math|Random|RandomFloatinRange 1.0 2e+04)) :!label _label_2)
      (Utilities|FlowControl|Delay (Math|Random|RandomFloatinRange 1.0 15.0))
      (goto _label_2))))

(fn ConstructionScript)