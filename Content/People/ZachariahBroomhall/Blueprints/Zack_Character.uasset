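; Spider AI character driven by a simple enum state machine with Idle, Walk, Berzerk and Death states, re-entered through ChangeState.
; Every Tick, a forward sphere trace stores any hit Character as LastSeenActor, which is never cleared.
; Once set, it moves Idle to random wandering, then to Berzerk.
; Berzerk plays roar and charge animations while timelines scale the capsule, then returns to Idle; Death destroys the actor, though nothing here sets it.
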(event Custom|CheckInFront
  ;[1 1 1] Sight
  (bind _outhit (Collision|SphereTraceForObjects (Transformation|GetActorLocation) (+ (Transformation|GetActorLocation) (* (Transformation|GetActorForwardVector) 5e+02)) 5e+03 (Utilities|Array|MakeArray "ObjectTypeQuery3") false 0 "ForOneFrame"))
  (bind _ascharacter (Utilities|Casting|CastToCharacter (.hitactor _outhit)))
  (Variables|Default|SetLastSeenActor _ascharacter))

(event Custom|Change%20State
  (switch Utilities|FlowControl|Switch|SwitchonZakStates (Variables|Default|Getcurrentstatus)
    (:NewEnumerator0
      ;[1 1 1] Berzerk (in Progress)
      (Components|Animation|PlayAnimation (Variables|Default|GetSkeletalMesh) "/Game/InfinityBladeAdversaries/Enemy/Enemy_Great_Spider/Enemy_SpiderGreater_Animation/ExoGame_Greater_Spider_Cast_Roar.ExoGame_Greater_Spider_Cast_Roar" false)
      (bind _track_1 (Timeline|Timeline%201 PlayFromStart)
        (:Update
          (Transformation|SetWorldScale3D (Variables|Collision|GetCapsuleComponent) (Math|Conversions|ToVector(Float) _track_1)))
        (:Finished
          (Components|Animation|PlayAnimation (Variables|Default|GetSkeletalMesh) "/Game/InfinityBladeAdversaries/Enemy/Enemy_Great_Spider/Enemy_SpiderGreater_Animation/ExoGame_Greater_Spider_Charge.ExoGame_Greater_Spider_Charge" false)
          (bind _newtrack_1 (Timeline|Timeline%202 PlayFromStart)
            (:Update
              (Transformation|SetWorldScale3D (Variables|Collision|GetCapsuleComponent) (Math|Conversions|ToVector(Float) _newtrack_1)))
            (:Finished
              (Utilities|FlowControl|Delay 3.0)
              (Variables|Default|Setcurrentstatus "NewEnumerator2")
              (CallFunction|ChangeState))))))
    (:NewEnumerator1
      ;[1 1 1] Wander
      (Components|Animation|PlayAnimation (Variables|Default|GetSkeletalMesh) "/Game/InfinityBladeAdversaries/Enemy/Enemy_Great_Spider/Enemy_SpiderGreater_Animation/ExoGame_Greater_Spider_Walk_Fwd.ExoGame_Greater_Spider_Walk_Fwd" true)
      (AI|Navigation|SimpleMovetoLocation (Pawn|GetController) (AI|Navigation|GetRandomReachablePointinRadius (Transformation|GetActorLocation) 1e+05))
      (Utilities|FlowControl|Delay (Math|Random|RandomFloat))
      (Utilities|IsValid (Variables|Default|GetLastSeenActor)
        (:Is%20Valid
          (Variables|Default|Setcurrentstatus "NewEnumerator0"))
        (:Is%20Not%20Valid
          (Variables|Default|Setcurrentstatus "NewEnumerator1")))
      (CallFunction|ChangeState))
    (:NewEnumerator2
      ;[1 1 1] Idle
      (Components|Animation|PlayAnimation (Variables|Default|GetSkeletalMesh) "/Game/InfinityBladeAdversaries/Enemy/Enemy_Great_Spider/Enemy_SpiderGreater_Animation/ExoGame_Greater_Spider_Idle.ExoGame_Greater_Spider_Idle" false)
      (Utilities|FlowControl|Delay 3.0)
      (Utilities|IsValid (Variables|Default|GetLastSeenActor)
        (:Is%20Valid
          (Variables|Default|Setcurrentstatus "NewEnumerator1")
          (CallFunction|ChangeState))
        (:Is%20Not%20Valid
          (Variables|Default|Setcurrentstatus "NewEnumerator2")
          (CallFunction|ChangeState))))
    (:NewEnumerator3
      ;[1 1 1] Death
      (Components|Animation|PlayAnimation (Variables|Default|GetSkeletalMesh) "/Game/InfinityBladeAdversaries/Enemy/Enemy_Great_Spider/Enemy_SpiderGreater_Animation/ExoGame_Greater_Spider_Death.ExoGame_Greater_Spider_Death" false)
      (Utilities|FlowControl|Delay 3.0)
      (Actor|DestroyActor))))

(event EventBeginPlay
  (switch Utilities|FlowControl|Switch|SwitchonZakStates (Variables|Default|Getcurrentstatus)
    (:NewEnumerator0
      ;[1 1 1] Berzerk (in Progress)
      (Components|Animation|PlayAnimation (Variables|Default|GetSkeletalMesh) "/Game/InfinityBladeAdversaries/Enemy/Enemy_Great_Spider/Enemy_SpiderGreater_Animation/ExoGame_Greater_Spider_Cast_Roar.ExoGame_Greater_Spider_Cast_Roar" false)
      (bind _track_1 (Timeline|Timeline%201 PlayFromStart)
        (:Update
          (Transformation|SetWorldScale3D (Variables|Collision|GetCapsuleComponent) (Math|Conversions|ToVector(Float) _track_1)))
        (:Finished
          (Components|Animation|PlayAnimation (Variables|Default|GetSkeletalMesh) "/Game/InfinityBladeAdversaries/Enemy/Enemy_Great_Spider/Enemy_SpiderGreater_Animation/ExoGame_Greater_Spider_Charge.ExoGame_Greater_Spider_Charge" false)
          (bind _newtrack_1 (Timeline|Timeline%202 PlayFromStart)
            (:Update
              (Transformation|SetWorldScale3D (Variables|Collision|GetCapsuleComponent) (Math|Conversions|ToVector(Float) _newtrack_1)))
            (:Finished
              (Utilities|FlowControl|Delay 3.0)
              (Variables|Default|Setcurrentstatus "NewEnumerator2")
              (CallFunction|ChangeState))))))
    (:NewEnumerator1
      ;[1 1 1] Wander
      (Components|Animation|PlayAnimation (Variables|Default|GetSkeletalMesh) "/Game/InfinityBladeAdversaries/Enemy/Enemy_Great_Spider/Enemy_SpiderGreater_Animation/ExoGame_Greater_Spider_Walk_Fwd.ExoGame_Greater_Spider_Walk_Fwd" true)
      (AI|Navigation|SimpleMovetoLocation (Pawn|GetController) (AI|Navigation|GetRandomReachablePointinRadius (Transformation|GetActorLocation) 1e+05))
      (Utilities|FlowControl|Delay (Math|Random|RandomFloat))
      (Utilities|IsValid (Variables|Default|GetLastSeenActor)
        (:Is%20Valid
          (Variables|Default|Setcurrentstatus "NewEnumerator0"))
        (:Is%20Not%20Valid
          (Variables|Default|Setcurrentstatus "NewEnumerator1")))
      (CallFunction|ChangeState))
    (:NewEnumerator2
      ;[1 1 1] Idle
      (Components|Animation|PlayAnimation (Variables|Default|GetSkeletalMesh) "/Game/InfinityBladeAdversaries/Enemy/Enemy_Great_Spider/Enemy_SpiderGreater_Animation/ExoGame_Greater_Spider_Idle.ExoGame_Greater_Spider_Idle" false)
      (Utilities|FlowControl|Delay 3.0)
      (Utilities|IsValid (Variables|Default|GetLastSeenActor)
        (:Is%20Valid
          (Variables|Default|Setcurrentstatus "NewEnumerator1")
          (CallFunction|ChangeState))
        (:Is%20Not%20Valid
          (Variables|Default|Setcurrentstatus "NewEnumerator2")
          (CallFunction|ChangeState))))
    (:NewEnumerator3
      ;[1 1 1] Death
      (Components|Animation|PlayAnimation (Variables|Default|GetSkeletalMesh) "/Game/InfinityBladeAdversaries/Enemy/Enemy_Great_Spider/Enemy_SpiderGreater_Animation/ExoGame_Greater_Spider_Death.ExoGame_Greater_Spider_Death" false)
      (Utilities|FlowControl|Delay 3.0)
      (Actor|DestroyActor))))

(event EventTick
  (params (DeltaSeconds :type Float%20%28single-precision%29))
  (CallFunction|CheckinFront))

(fn ConstructionScript)