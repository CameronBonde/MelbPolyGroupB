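; Dude is a character that plays bear animations through a simple state machine of Dead, Idle, Walk and Spin.
; BeginPlay and UpdateState share one switch on CurrentState, which plays animations directly on the mesh and uses delays to re-evaluate.
; Idle repeats and Walk leads to Dead.
; Spin rotates the capsule via a timeline, then plays a random melee attack; its return-to-Idle chain is unconnected.
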(event Custom|Update%20state
  (bind _mesh (Variables|Character|GetMesh))
  (switch Utilities|FlowControl|Switch|SwitchonDudeStates (Variables|Default|GetCurrent%20state)
    (:NewEnumerator0
      ;[1 1 1] Dead
      (Components|Animation|PlayAnimation (Variables|Character|GetMesh) "/Game/InfinityBladeAdversaries/Enemy/Enemy_Bear/Enemy_Bear_Animations/ExoGame_Bears_Attack_Death.ExoGame_Bears_Attack_Death" false))
    (:NewEnumerator1
      ;[1 1 1] Idle
      (Components|Animation|PlayAnimation (Variables|Character|GetMesh) "/Game/InfinityBladeAdversaries/Enemy/Enemy_Bear/Enemy_Bear_Animations/ExoGame_Bears_Idle.ExoGame_Bears_Idle" true)
      (Utilities|FlowControl|Delay 4.0)
      (CallFunction|UpdateState))
    (:NewEnumerator2
      ;[1 1 1] Walking
      (Components|Animation|PlayAnimation (Variables|Character|GetMesh) "/Game/InfinityBladeAdversaries/Enemy/Enemy_Bear/Enemy_Bear_Animations/ExoGame_Bears_Walk.ExoGame_Bears_Walk" true)
      (Utilities|FlowControl|Delay 4.0)
      (Variables|Default|SetCurrent%20state "NewEnumerator0")
      (CallFunction|UpdateState))
    (:NewEnumerator4
      ;[1 1 1] Spin attack
      (Components|Animation|PlayAnimation (Variables|Character|GetMesh) "/Game/InfinityBladeAdversaries/Enemy/Enemy_Bear/Enemy_Bear_Animations/ExoGame_Bears_Drop_Down.ExoGame_Bears_Drop_Down" false)
      (Utilities|FlowControl|Delay 2.0)
      (Timeline|Timeline_0 PlayFromStart
        (:Update
          (Transformation|AddLocalRotation (Variables|Collision|GetCapsuleComponent) "0,2.000000, 0" false false))
        (:Finished
          (if (Math|Random|RandomBool)
            (Components|Animation|PlayAnimation _mesh "/Game/InfinityBladeAdversaries/Enemy/Enemy_Bear/Enemy_Bear_Animations/ExoGame_Bears_Attack_Melee.ExoGame_Bears_Attack_Melee" false)
            (else
              (Components|Animation|PlayAnimation _mesh "/Game/InfinityBladeAdversaries/Enemy/Enemy_Bear/Enemy_Bear_Animations/ExoGame_Bears_Attack_Melee_B.ExoGame_Bears_Attack_Melee_B" false))))))))

(event EventBeginPlay
  (bind _mesh (Variables|Character|GetMesh))
  (switch Utilities|FlowControl|Switch|SwitchonDudeStates (Variables|Default|GetCurrent%20state)
    (:NewEnumerator0
      ;[1 1 1] Dead
      (Components|Animation|PlayAnimation (Variables|Character|GetMesh) "/Game/InfinityBladeAdversaries/Enemy/Enemy_Bear/Enemy_Bear_Animations/ExoGame_Bears_Attack_Death.ExoGame_Bears_Attack_Death" false))
    (:NewEnumerator1
      ;[1 1 1] Idle
      (Components|Animation|PlayAnimation (Variables|Character|GetMesh) "/Game/InfinityBladeAdversaries/Enemy/Enemy_Bear/Enemy_Bear_Animations/ExoGame_Bears_Idle.ExoGame_Bears_Idle" true)
      (Utilities|FlowControl|Delay 4.0)
      (CallFunction|UpdateState))
    (:NewEnumerator2
      ;[1 1 1] Walking
      (Components|Animation|PlayAnimation (Variables|Character|GetMesh) "/Game/InfinityBladeAdversaries/Enemy/Enemy_Bear/Enemy_Bear_Animations/ExoGame_Bears_Walk.ExoGame_Bears_Walk" true)
      (Utilities|FlowControl|Delay 4.0)
      (Variables|Default|SetCurrent%20state "NewEnumerator0")
      (CallFunction|UpdateState))
    (:NewEnumerator4
      ;[1 1 1] Spin attack
      (Components|Animation|PlayAnimation (Variables|Character|GetMesh) "/Game/InfinityBladeAdversaries/Enemy/Enemy_Bear/Enemy_Bear_Animations/ExoGame_Bears_Drop_Down.ExoGame_Bears_Drop_Down" false)
      (Utilities|FlowControl|Delay 2.0)
      (Timeline|Timeline_0 PlayFromStart
        (:Update
          (Transformation|AddLocalRotation (Variables|Collision|GetCapsuleComponent) "0,2.000000, 0" false false))
        (:Finished
          (if (Math|Random|RandomBool)
            (Components|Animation|PlayAnimation _mesh "/Game/InfinityBladeAdversaries/Enemy/Enemy_Bear/Enemy_Bear_Animations/ExoGame_Bears_Attack_Melee.ExoGame_Bears_Attack_Melee" false)
            (else
              (Components|Animation|PlayAnimation _mesh "/Game/InfinityBladeAdversaries/Enemy/Enemy_Bear/Enemy_Bear_Animations/ExoGame_Bears_Attack_Melee_B.ExoGame_Bears_Attack_Melee_B" false))))))))

(fn ConstructionScript)