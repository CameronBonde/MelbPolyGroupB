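; CameronBonde is an AI character driven by an enum state machine, re-entered through UpdateStates after each action.
; Tick box-traces forward to remember the last Character seen, which steers wandering, following fellow CameronBondes and fleeing.
; Teleport (sink, then reappear at a random reachable point) and line-of-sight attack (effect, then damage call) states loop on themselves.
; Damage feeds the Health component, whose death event triggers the Dead animation and destroys the actor.
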(event OnDeath(Health)
  (Variables|Default|SetCurrent%20State "NewEnumerator5")
  (CallFunction|UpdateStates))

(event Custom|Update%20senses
  ;[1 1 1] Sight
  (bind _outhit (Collision|BoxTraceByChannel (Transformation|GetActorLocation) (+ (Transformation|GetActorLocation) (* (Transformation|GetActorForwardVector) 2e+03)) "200.000000,200.000000,50.000000" "0, 0, 0" "TraceTypeQuery2" false 0 "None"))
  ;[1 1 1] Check if we hit any other 'character'
  (bind _ascharacter (Utilities|Casting|CastToCharacter (.hitactor _outhit)))
  ;[1 1 1] Remember last actor
  (Variables|Default|SetLast%20seen%20actor _ascharacter))

(event Custom|Update%20states
  (switch Utilities|FlowControl|Switch|SwitchonCameronBondeStates (Variables|Default|GetCurrent%20State)
    (:NewEnumerator1
      ;[1 1 1] Follow buddy
      (Utilities|FlowControl|Delay (Math|Random|RandomFloatinRange 1.0 2.0))
      (AI|Navigation|SimpleMovetoLocation (Pawn|GetController) (Transformation|GetActorLocation (Variables|Default|GetLast%20seen%20actor)))
      ;[1 1 1] Change state when Enemy is about
      (Utilities|Casting|CastToCameronBonde (Variables|Default|GetLast%20seen%20actor)
        (:then
          (CallFunction|UpdateStates))
        (:CastFailed
          (Variables|Default|SetCurrent%20State "NewEnumerator0")
          (CallFunction|UpdateStates))))
    (:NewEnumerator0
      ;[1 1 1] Randomly walk about
      ;;[1 1 1] Pick a random location
      (AI|AIMoveTo (Class|CharacterMovementComponent|GetCharacterOwner (Variables|Character|GetCharacterMovement)) (AI|Navigation|GetRandomReachablePointinRadius (Transformation|GetActorLocation) 1e+04) 0 5.0 false
        (:OnSuccess
          (Utilities|FlowControl|Delay (Math|Random|RandomFloatinRange 1.0 2.0))
          ;[1 1 1] Seen a buddy, Change state to Move toward buddy
          (Utilities|Casting|CastToCameronBonde (Variables|Default|GetLast%20seen%20actor)
            (:then
              (Variables|Default|SetCurrent%20State "NewEnumerator1")
              (CallFunction|UpdateStates))
            (:CastFailed
              ;[1 1 1] Change state to Run away
              (Variables|Default|SetCurrent%20State "NewEnumerator3")
              (CallFunction|UpdateStates))))))
    (:NewEnumerator2
      ;[1 1 1] Teleport
      (Collision|SetCollisionEnabled (Variables|Collision|GetCapsuleComponent) "NoCollision")
      (Timeline|Sink%20into%20ground PlayFromStart
        (:Update
          (Transformation|AddRelativeLocation (Variables|Collision|GetCapsuleComponent) "0, 0,-1.000000" false false))
        (:Finished
          (Transformation|SetActorLocation (+ (AI|Navigation|GetRandomReachablePointinRadius (Transformation|GetActorLocation) 1e+04) "0, 0,500.000000") false true)
          (Collision|SetCollisionEnabled (Variables|Collision|GetCapsuleComponent) "QueryAndPhysics")
          (Utilities|FlowControl|Delay 2.0)
          (Variables|Default|SetCurrent%20State "NewEnumerator2")
          (CallFunction|UpdateStates))))
    (:NewEnumerator3
      ;[1 1 1] Run away
      (Utilities|IsValid (Variables|Default|GetLast%20seen%20actor) ; Check to see if he's seen anything yet
        (:Is%20Valid
          (if (< (Transformation|GetDistanceTo (Variables|Default|GetLast%20seen%20actor)) (Variables|Default|GetMinimumAttackDistance))
            (AI|AIMoveTo (Class|PawnMovementComponent|GetPawnOwner (Variables|Character|GetCharacterMovement)) (+ (* (Math|Vector|Normalize (- (Transformation|GetActorLocation) (Transformation|GetActorLocation (Variables|Default|GetLast%20seen%20actor)))) (Variables|Default|GetMinimumAttackDistance)) (Transformation|GetActorLocation (Variables|Default|GetLast%20seen%20actor))) 0 5.0 false
              (:OnSuccess
                (Variables|Default|SetCurrent%20State "NewEnumerator0")
                (CallFunction|UpdateStates)))
            (else
              (Utilities|FlowControl|Delay 0.2 :!label _label)
              (Variables|Default|SetCurrent%20State "NewEnumerator0")
              (CallFunction|UpdateStates))))
        (:Is%20Not%20Valid
          (goto _label))))
    (:NewEnumerator4
      ;[1 1 1] Line of sight damage
      (Components|Animation|PlayAnimation (Variables|Character|GetMesh) "/Game/InfinityBladeAdversaries/Enemy/Enemy_Gruntling/Enemy_Gruntling_Animation/ExoGame_Gruntling_Cast.ExoGame_Gruntling_Cast" false)
      (Utilities|FlowControl|Delay 0.75)
      (Audio|Components|Audio|Stop (Variables|Character|GetMesh))
      (bind _returnvalue (Game|SpawnActorfromClass "/Game/People/CameronBonde/Blueprints/SuperCoolEffect.SuperCoolEffect_C" (Transformation|GetWorldTransform (Variables|Default|GetEffect%20spawn%20point)) "Undefined" 0 0))
      (Variables|Default|SetLOSEffect _returnvalue)
      (Timeline|Check%20for%20enemy PlayFromStart ; TODO: Check for enemy
        (:Finished
          (Game|Damage|ApplyDamage (Variables|Default|GetLast%20seen%20actor) 0.0 0 0) ; TODO: Only for enemies
          (Actor|DestroyActor (Variables|Default|GetLOSEffect))
          (Components|Animation|PlayAnimation (Variables|Character|GetMesh) "/Game/InfinityBladeAdversaries/Enemy/Enemy_Gruntling/Enemy_Gruntling_Animation/ExoGame_Gruntling_Cast.ExoGame_Gruntling_Cast" false)
          (Utilities|FlowControl|Delay 1.0)
          (Variables|Default|SetCurrent%20State "NewEnumerator4")
          (CallFunction|UpdateStates))))
    (:NewEnumerator5
      ;[1 1 1] Death
      (Components|Animation|PlayAnimation (Variables|Character|GetMesh) "/Game/InfinityBladeAdversaries/Enemy/Enemy_Gruntling/Enemy_Gruntling_Animation/ExoGame_Gruntling_Death.ExoGame_Gruntling_Death" false)
      (Utilities|FlowControl|Delay 1.0)
      (Actor|DestroyActor))))

(event EventBeginPlay
  (switch Utilities|FlowControl|Switch|SwitchonCameronBondeStates (Variables|Default|GetCurrent%20State)
    (:NewEnumerator1
      ;[1 1 1] Follow buddy
      (Utilities|FlowControl|Delay (Math|Random|RandomFloatinRange 1.0 2.0))
      (AI|Navigation|SimpleMovetoLocation (Pawn|GetController) (Transformation|GetActorLocation (Variables|Default|GetLast%20seen%20actor)))
      ;[1 1 1] Change state when Enemy is about
      (Utilities|Casting|CastToCameronBonde (Variables|Default|GetLast%20seen%20actor)
        (:then
          (CallFunction|UpdateStates))
        (:CastFailed
          (Variables|Default|SetCurrent%20State "NewEnumerator0")
          (CallFunction|UpdateStates))))
    (:NewEnumerator0
      ;[1 1 1] Randomly walk about
      ;;[1 1 1] Pick a random location
      (AI|AIMoveTo (Class|CharacterMovementComponent|GetCharacterOwner (Variables|Character|GetCharacterMovement)) (AI|Navigation|GetRandomReachablePointinRadius (Transformation|GetActorLocation) 1e+04) 0 5.0 false
        (:OnSuccess
          (Utilities|FlowControl|Delay (Math|Random|RandomFloatinRange 1.0 2.0))
          ;[1 1 1] Seen a buddy, Change state to Move toward buddy
          (Utilities|Casting|CastToCameronBonde (Variables|Default|GetLast%20seen%20actor)
            (:then
              (Variables|Default|SetCurrent%20State "NewEnumerator1")
              (CallFunction|UpdateStates))
            (:CastFailed
              ;[1 1 1] Change state to Run away
              (Variables|Default|SetCurrent%20State "NewEnumerator3")
              (CallFunction|UpdateStates))))))
    (:NewEnumerator2
      ;[1 1 1] Teleport
      (Collision|SetCollisionEnabled (Variables|Collision|GetCapsuleComponent) "NoCollision")
      (Timeline|Sink%20into%20ground PlayFromStart
        (:Update
          (Transformation|AddRelativeLocation (Variables|Collision|GetCapsuleComponent) "0, 0,-1.000000" false false))
        (:Finished
          (Transformation|SetActorLocation (+ (AI|Navigation|GetRandomReachablePointinRadius (Transformation|GetActorLocation) 1e+04) "0, 0,500.000000") false true)
          (Collision|SetCollisionEnabled (Variables|Collision|GetCapsuleComponent) "QueryAndPhysics")
          (Utilities|FlowControl|Delay 2.0)
          (Variables|Default|SetCurrent%20State "NewEnumerator2")
          (CallFunction|UpdateStates))))
    (:NewEnumerator3
      ;[1 1 1] Run away
      (Utilities|IsValid (Variables|Default|GetLast%20seen%20actor) ; Check to see if he's seen anything yet
        (:Is%20Valid
          (if (< (Transformation|GetDistanceTo (Variables|Default|GetLast%20seen%20actor)) (Variables|Default|GetMinimumAttackDistance))
            (AI|AIMoveTo (Class|PawnMovementComponent|GetPawnOwner (Variables|Character|GetCharacterMovement)) (+ (* (Math|Vector|Normalize (- (Transformation|GetActorLocation) (Transformation|GetActorLocation (Variables|Default|GetLast%20seen%20actor)))) (Variables|Default|GetMinimumAttackDistance)) (Transformation|GetActorLocation (Variables|Default|GetLast%20seen%20actor))) 0 5.0 false
              (:OnSuccess
                (Variables|Default|SetCurrent%20State "NewEnumerator0")
                (CallFunction|UpdateStates)))
            (else
              (Utilities|FlowControl|Delay 0.2 :!label _label)
              (Variables|Default|SetCurrent%20State "NewEnumerator0")
              (CallFunction|UpdateStates))))
        (:Is%20Not%20Valid
          (goto _label))))
    (:NewEnumerator4
      ;[1 1 1] Line of sight damage
      (Components|Animation|PlayAnimation (Variables|Character|GetMesh) "/Game/InfinityBladeAdversaries/Enemy/Enemy_Gruntling/Enemy_Gruntling_Animation/ExoGame_Gruntling_Cast.ExoGame_Gruntling_Cast" false)
      (Utilities|FlowControl|Delay 0.75)
      (Audio|Components|Audio|Stop (Variables|Character|GetMesh))
      (bind _returnvalue (Game|SpawnActorfromClass "/Game/People/CameronBonde/Blueprints/SuperCoolEffect.SuperCoolEffect_C" (Transformation|GetWorldTransform (Variables|Default|GetEffect%20spawn%20point)) "Undefined" 0 0))
      (Variables|Default|SetLOSEffect _returnvalue)
      (Timeline|Check%20for%20enemy PlayFromStart ; TODO: Check for enemy
        (:Finished
          (Game|Damage|ApplyDamage (Variables|Default|GetLast%20seen%20actor) 0.0 0 0) ; TODO: Only for enemies
          (Actor|DestroyActor (Variables|Default|GetLOSEffect))
          (Components|Animation|PlayAnimation (Variables|Character|GetMesh) "/Game/InfinityBladeAdversaries/Enemy/Enemy_Gruntling/Enemy_Gruntling_Animation/ExoGame_Gruntling_Cast.ExoGame_Gruntling_Cast" false)
          (Utilities|FlowControl|Delay 1.0)
          (Variables|Default|SetCurrent%20State "NewEnumerator4")
          (CallFunction|UpdateStates))))
    (:NewEnumerator5
      ;[1 1 1] Death
      (Components|Animation|PlayAnimation (Variables|Character|GetMesh) "/Game/InfinityBladeAdversaries/Enemy/Enemy_Gruntling/Enemy_Gruntling_Animation/ExoGame_Gruntling_Death.ExoGame_Gruntling_Death" false)
      (Utilities|FlowControl|Delay 1.0)
      (Actor|DestroyActor))))

(event Game|Damage|EventAnyDamage
  (params (Damage :type Float%20%28single-precision%29) (DamageType :type Damage%20Type%20Object%20Reference) (InstigatedBy :type Controller%20Object%20Reference) (DamageCauser :type Actor%20Object%20Reference))
  (Default|ChangeHealth (Variables|Default|GetHealth) (Math|Float|Truncate Damage) false))

(event EventTick
  (params (DeltaSeconds :type Float%20%28single-precision%29))
  ;[1 1 1] Main loop
  (CallFunction|UpdateSenses))

(fn ConstructionScript)