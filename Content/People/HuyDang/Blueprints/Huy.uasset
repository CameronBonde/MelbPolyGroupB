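; Huy is an AI-moved pawn or character that wanders around, driven each Tick by a sensing trace and a switch on CurrentState.
; Walking Around moves it to a random reachable point after a one-second delay, while Get Rekt only prints a message.
; Lenses casts a debug-drawn forward box trace, but its result is unused, and nothing here changes the state.
; Med is a stub that prints a greeting.
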(event Custom|Med
  (Development|PrintString "Hello"))

(event Custom|Lenses
  ;[1 1 1] Senses
  (bind _outhit (Collision|BoxTraceByChannel (Transformation|GetActorLocation) (+ (Transformation|GetActorLocation) (* (Transformation|GetActorForwardVector) 1e+04)) "200.000000,200.000000,200.000000" (Pawn|GetControlRotation :!class /Script/Engine.Pawn) "TraceTypeQuery2" false 0 "ForOneFrame")))

(event Custom|UpdateState
  (switch Utilities|FlowControl|Switch|SwitchonHuys_new_Enumaeration (Variables|Default|GetCurrent%20State)
    (:NewEnumerator0
      ;[1 1 1] Movement
      (Utilities|FlowControl|Delay (Math|Random|RandomFloatinRange 1.0 1.0))
      (AI|Navigation|SimpleMovetoLocation (Pawn|GetController) (AI|Navigation|GetRandomReachablePointinRadius (Transformation|GetActorLocation) 1e+04)))
    (:NewEnumerator2
      (Development|PrintString "Du Ma"))))

(event EventTick
  (params (DeltaSeconds :type Float%20%28single-precision%29))
  (CallFunction|Lenses)
  (CallFunction|UpdateState))

(fn ConstructionScript)