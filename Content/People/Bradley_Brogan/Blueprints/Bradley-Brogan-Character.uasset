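; Bradley Brogan character Blueprint for an NPC that wanders at random.
; BeginPlay starts an endless loop that sends the controller to a random reachable point near the actor, then waits a short random delay before repeating.
; A CheckInFront event box-traces the Visibility channel far along the forward vector, but nothing in the graph calls it or uses its result.
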(event Custom|CheckInFront
  ;[1 1 1] Senses
  (Collision|BoxTraceByChannel (Transformation|GetActorLocation) (+ (Transformation|GetActorLocation) (* (Transformation|GetActorForwardVector) 1e+04)) "0, 0, 0" "0, 0, 0" "TraceTypeQuery1" false 0 "None"))

(event EventBeginPlay
  ;[1 1 1] Walk around
  (AI|Navigation|SimpleMovetoLocation (Pawn|GetController) (AI|Navigation|GetRandomReachablePointinRadius (Transformation|GetActorLocation) 1e+03) :!label _label)
  (Utilities|FlowControl|Delay (Math|Random|RandomFloatinRange 1.0 4.0))
  (goto _label))

(fn ConstructionScript)