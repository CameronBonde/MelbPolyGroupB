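; Clot worm AI character that idles, wanders and flees from characters it spots.
; A per-tick forward box trace stores any hit Character as LastSeenActor, which is never cleared here.
; An enum state machine, re-entered through UpdateState, plays animations and moves to random reachable points or away from that actor.
; Damage feeds the Health component; the Death state animates then destroys the worm, but nothing here sets it.
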(event Custom|Update%20State
  (switch Utilities|FlowControl|Switch|SwitchonBradleyBroganStates (Variables|Default|GetCurrent%20State)
    (:NewEnumerator0
      ;[1 1 1] Death
      (Components|Animation|PlayAnimation (Variables|Character|GetMesh) "/Game/InfinityBladeAdversaries/Enemy/Enemy_Clot_Worm/Enemy_Clot_Worm_Animation/ExoGame_Clot_Worm_Death_1.ExoGame_Clot_Worm_Death_1" false)
      (Utilities|FlowControl|Delay 4.0)
      (Actor|DestroyActor))
    (:NewEnumerator1
      ;[1 1 1] Idle
      (Components|Animation|PlayAnimation (Variables|Character|GetMesh) "/Game/InfinityBladeAdversaries/Enemy/Enemy_Clot_Worm/Enemy_Clot_Worm_Animation/ExoGame_Baby_Clot_Worm_Idle.ExoGame_Baby_Clot_Worm_Idle" true)
      (Utilities|FlowControl|Delay 2.0)
      (Variables|Default|SetCurrent%20State "NewEnumerator2")
      (CallFunction|UpdateState))
    (:NewEnumerator2
      ;[1 1 1] Walk/Slither
      (Components|Animation|PlayAnimation (Variables|Character|GetMesh) "/Game/InfinityBladeAdversaries/Enemy/Enemy_Clot_Worm/Enemy_Clot_Worm_Animation/ExoGame_Baby_Clot_Worm_Slither_Foreward.ExoGame_Baby_Clot_Worm_Slither_Foreward" true)
      (AI|Navigation|SimpleMovetoLocation (Pawn|GetController) (AI|Navigation|GetRandomReachablePointinRadius (Transformation|GetActorLocation) 1e+04))
      (Utilities|FlowControl|Delay 2.0)
      (Utilities|IsValid (Variables|Default|GetLast%20seen%20actor)
        (:Is%20Valid
          ;[1 1 1] Change State to Runaway
          (Variables|Default|SetCurrent%20State "NewEnumerator5")
          (CallFunction|UpdateState))
        (:Is%20Not%20Valid
          ;[1 1 1] Keep Walking
          (Variables|Default|SetCurrent%20State "NewEnumerator2")
          (CallFunction|UpdateState))))
    (:NewEnumerator5
      ;[1 1 1] Run Away
      (Components|Animation|PlayAnimation (Variables|Character|GetMesh) "/Game/InfinityBladeAdversaries/Enemy/Enemy_Clot_Worm/Enemy_Clot_Worm_Animation/ExoGame_Baby_Clot_Worm_Slither_Foreward.ExoGame_Baby_Clot_Worm_Slither_Foreward" false)
      (AI|AIMoveTo (Class|CharacterMovementComponent|GetCharacterOwner (Variables|Character|GetCharacterMovement)) (+ (Transformation|GetActorLocation (Variables|Default|GetLast%20seen%20actor)) (* (Math|Vector|Normalize (- (Transformation|GetActorLocation) (Transformation|GetActorLocation (Variables|Default|GetLast%20seen%20actor)))) (Transformation|GetActorLocation))) 0 5.0 false
        (:OnSuccess
          (Utilities|IsValid (Variables|Default|GetLast%20seen%20actor)
            (:Is%20Valid
              ;[1 1 1] Keep running away
              (Variables|Default|SetCurrent%20State "NewEnumerator5")
              (CallFunction|UpdateState))
            (:Is%20Not%20Valid
              ;[1 1 1] go back to Walking around
              (Variables|Default|SetCurrent%20State "NewEnumerator2")
              (CallFunction|UpdateState))))))))

(event Custom|CheckinFront
  ;[1 1 1] Sight
  (bind _outhit (Collision|BoxTraceByChannel (Transformation|GetActorLocation) (+ (Transformation|GetActorLocation) (* (Transformation|GetActorForwardVector) 2e+03)) "200.000000,200.000000,50.000000" "0, 0, 0" "TraceTypeQuery2" false 0 "ForOneFrame"))
  (bind _ascharacter (Utilities|Casting|CastToCharacter (.hitactor _outhit)))
  (Variables|Default|SetLast%20seen%20actor _ascharacter))

(event EventBeginPlay
  (switch Utilities|FlowControl|Switch|SwitchonBradleyBroganStates (Variables|Default|GetCurrent%20State)
    (:NewEnumerator0
      ;[1 1 1] Death
      (Components|Animation|PlayAnimation (Variables|Character|GetMesh) "/Game/InfinityBladeAdversaries/Enemy/Enemy_Clot_Worm/Enemy_Clot_Worm_Animation/ExoGame_Clot_Worm_Death_1.ExoGame_Clot_Worm_Death_1" false)
      (Utilities|FlowControl|Delay 4.0)
      (Actor|DestroyActor))
    (:NewEnumerator1
      ;[1 1 1] Idle
      (Components|Animation|PlayAnimation (Variables|Character|GetMesh) "/Game/InfinityBladeAdversaries/Enemy/Enemy_Clot_Worm/Enemy_Clot_Worm_Animation/ExoGame_Baby_Clot_Worm_Idle.ExoGame_Baby_Clot_Worm_Idle" true)
      (Utilities|FlowControl|Delay 2.0)
      (Variables|Default|SetCurrent%20State "NewEnumerator2")
      (CallFunction|UpdateState))
    (:NewEnumerator2
      ;[1 1 1] Walk/Slither
      (Components|Animation|PlayAnimation (Variables|Character|GetMesh) "/Game/InfinityBladeAdversaries/Enemy/Enemy_Clot_Worm/Enemy_Clot_Worm_Animation/ExoGame_Baby_Clot_Worm_Slither_Foreward.ExoGame_Baby_Clot_Worm_Slither_Foreward" true)
      (AI|Navigation|SimpleMovetoLocation (Pawn|GetController) (AI|Navigation|GetRandomReachablePointinRadius (Transformation|GetActorLocation) 1e+04))
      (Utilities|FlowControl|Delay 2.0)
      (Utilities|IsValid (Variables|Default|GetLast%20seen%20actor)
        (:Is%20Valid
          ;[1 1 1] Change State to Runaway
          (Variables|Default|SetCurrent%20State "NewEnumerator5")
          (CallFunction|UpdateState))
        (:Is%20Not%20Valid
          ;[1 1 1] Keep Walking
          (Variables|Default|SetCurrent%20State "NewEnumerator2")
          (CallFunction|UpdateState))))
    (:NewEnumerator5
      ;[1 1 1] Run Away
      (Components|Animation|PlayAnimation (Variables|Character|GetMesh) "/Game/InfinityBladeAdversaries/Enemy/Enemy_Clot_Worm/Enemy_Clot_Worm_Animation/ExoGame_Baby_Clot_Worm_Slither_Foreward.ExoGame_Baby_Clot_Worm_Slither_Foreward" false)
      (AI|AIMoveTo (Class|CharacterMovementComponent|GetCharacterOwner (Variables|Character|GetCharacterMovement)) (+ (Transformation|GetActorLocation (Variables|Default|GetLast%20seen%20actor)) (* (Math|Vector|Normalize (- (Transformation|GetActorLocation) (Transformation|GetActorLocation (Variables|Default|GetLast%20seen%20actor)))) (Transformation|GetActorLocation))) 0 5.0 false
        (:OnSuccess
          (Utilities|IsValid (Variables|Default|GetLast%20seen%20actor)
            (:Is%20Valid
              ;[1 1 1] Keep running away
              (Variables|Default|SetCurrent%20State "NewEnumerator5")
              (CallFunction|UpdateState))
            (:Is%20Not%20Valid
              ;[1 1 1] go back to Walking around
              (Variables|Default|SetCurrent%20State "NewEnumerator2")
              (CallFunction|UpdateState))))))))

(event EventTick
  (params (DeltaSeconds :type Float%20%28single-precision%29))
  ;[1 1 1] Sight Loop
  (CallFunction|CheckinFront))

(event Game|Damage|EventAnyDamage
  (params (Damage :type Float%20%28single-precision%29) (DamageType :type Damage%20Type%20Object%20Reference) (InstigatedBy :type Controller%20Object%20Reference) (DamageCauser :type Actor%20Object%20Reference))
  (Default|ChangeHealth (Variables|Default|GetHealth) (Math|Float|Truncate Damage)))

(fn ConstructionScript)